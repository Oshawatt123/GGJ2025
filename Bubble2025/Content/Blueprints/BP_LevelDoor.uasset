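; BP_LevelDoor is an interactable door that loads the level named in LevelToLoad.
; On Interact it calls the parent's Interact, then finds the BP_StoryBubble actor in the world and checks its LevelLoadReady flag.
; When the flag is set, it waits briefly and opens the level by name, so the story bubble gates travel through the door.
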(event `/Game/Blueprints/BPI_Interactable.Interact`
  (`parent.Interact`)
  (bind _returnvalue (`GameplayStatics.GetActorOfClass` "/Game/Blueprints/BP_StoryBubble.BP_StoryBubble_C"))
  (if (`/Game/Blueprints/BP_StoryBubble.LevelLoadReady` _returnvalue)
    (`KismetSystemLibrary.Delay` 0.2)
    (`GameplayStatics.OpenLevel` (`self.LevelToLoad`))))

(fn `UserConstructionScript`
  (`parent.UserConstructionScript`))