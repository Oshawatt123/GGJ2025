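; Entity actor that distorts the screen and plays audio when the player gets close, with placeholder-like garbled dialogue text set on BeginPlay.
; Every tick it compares the player's distance to its skeletal mesh against CameraEffectRadius.
; Inside the radius it switches post process volumes tagged PP_Entity on and PP_Default off and starts its audio; outside, it reverses both and stops the audio.
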(event `self.ReceiveBeginPlay`
  (`parent.ReceiveBeginPlay`)
  (set `self.ObjectDialogue` "!??!!!?!?!?!?!?!!?!")
  (bind _outactors (`GameplayStatics.GetAllActorsWithTag` "PP_Entity"))
  (for _array_element _outactors
    (bind _aspost_process_volume (cast `PostProcessVolume` _array_element))
    (set `PostProcessVolume.BlendWeight` 0.0 _aspost_process_volume)))

(event `self.ReceiveTick`
  (params (DeltaSeconds :type "Float (single-precision)"))
  (bind _audio (`self.Audio`))
  (`parent.ReceiveTick` DeltaSeconds)
  (if (< (`KismetMathLibrary.Vector_Distance` (`self.K2_GetActorLocation` (`GameplayStatics.GetPlayerCharacter` 0)) (`SceneComponent.K2_GetComponentLocation` (`self.SkeletalMesh`))) (`self.CameraEffectRadius`))
    (bind _outactors (`GameplayStatics.GetAllActorsWithTag` "PP_Entity"))
    (for _array_element _outactors
      (bind _aspost_process_volume (cast `PostProcessVolume` _array_element))
      (set `PostProcessVolume.BlendWeight` 1.0 _aspost_process_volume))
    (bind _outactors_2 (`GameplayStatics.GetAllActorsWithTag` "PP_Default"))
    (for _array_element_2 _outactors_2
      (bind _aspost_process_volume_2 (cast `PostProcessVolume` _array_element_2))
      (set `PostProcessVolume.BlendWeight` 0.0 _aspost_process_volume_2))
    (if (not (`AudioComponent.IsPlaying` _audio))
      (`AudioComponent.Play` _audio 0.0))
    (else
      (bind _outactors_3 (`GameplayStatics.GetAllActorsWithTag` "PP_Default"))
      (for _array_element_3 _outactors_3
        (bind _aspost_process_volume_3 (cast `PostProcessVolume` _array_element_3))
        (set `PostProcessVolume.BlendWeight` 1.0 _aspost_process_volume_3))
      (bind _outactors_4 (`GameplayStatics.GetAllActorsWithTag` "PP_Entity"))
      (for _array_element_4 _outactors_4
        (bind _aspost_process_volume_4 (cast `PostProcessVolume` _array_element_4))
        (set `PostProcessVolume.BlendWeight` 0.0 _aspost_process_volume_4))
      (`AudioComponent.Stop` (`self.Audio`)))))

(fn `UserConstructionScript`
  (`parent.UserConstructionScript`))