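; Manager that periodically relocates the level's single BP_Entity among BP_EntityPoint actors near the player.
; A self-rearming random timer first parks the entity far away for an optional despawn delay, then moves it and yaws it toward the player.
; GetEntitySpawnPoint picks randomly from points within SpawnRadius, excluding CurrentPoint, or returns an off-map location if none qualify.
; Separate Random calls set CurrentPoint and the returned location, so they can differ.
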(event `self.ReceiveBeginPlay`
  (bind _outactors (`GameplayStatics.GetAllActorsOfClass` "/Game/Blueprints/BP_EntityPoint.BP_EntityPoint_C"))
  (set `self.points` _outactors)
  (`KismetSystemLibrary.K2_SetTimerDelegate` (delegate `SpawnEntity`) (`KismetMathLibrary.RandomFloatInRange` (`self.SpawnTimeMin`) (`self.SpawnTimeMax`)))
  (bind _returnvalue (`GameplayStatics.GetActorOfClass` "/Game/Blueprints/BP_Entity.BP_Entity_C"))
  (set `self.Entity` _returnvalue))

(event `SpawnEntity`
  (bind _entity (`self.Entity`))
  (if (not (== (`self.DespawnDelay`) 0.0))
    (`self.K2_SetActorLocation` (`self.Entity`) (0.0 -10000.0 0.0) false false)
    (`KismetSystemLibrary.Delay` (`self.DespawnDelay`)))
  (bind _newparam (`self.GetEntitySpawnPoint`))
  (`self.K2_SetActorLocation` _entity _newparam false false)
  (bind (_returnvalue_roll _returnvalue_pitch _returnvalue_yaw) (`KismetMathLibrary.BreakRotator` (`KismetMathLibrary.FindLookAtRotation` _newparam (`SceneComponent.K2_GetComponentLocation` (`Character.CapsuleComponent` (`GameplayStatics.GetPlayerCharacter` 0))))))
  (`self.K2_SetActorRotation` _entity (`KismetMathLibrary.MakeRotator` 0.0 0.0 _returnvalue_yaw) false)
  (`KismetSystemLibrary.K2_SetTimerDelegate` (delegate `SpawnEntity`) (`KismetMathLibrary.RandomFloatInRange` (`self.SpawnTimeMin`) (`self.SpawnTimeMax`))))

(fn `GetEntitySpawnPoint`
  (returns (NewParam :type "Vector Structure"))
  (locals (PointsCopy :type "Array of /Game/Blueprints/BP_EntityPoint Object Reference") (ValidPoints :type "Array of /Game/Blueprints/BP_EntityPoint Object Reference"))
  (bind _pointscopy (`local.PointsCopy`))
  (bind _validpoints (`local.ValidPoints`))
  (bind _outitem (`KismetArrayLibrary.Array_Random` _validpoints))
  (set `local.PointsCopy` (`self.points`))
  (bind _currentpoint (`self.CurrentPoint`)
    (:`then`
      (`KismetArrayLibrary.Array_RemoveItem` _pointscopy _currentpoint))
    (:`else`
      _))
  (for _array_element _pointscopy
    (if (< (`KismetMathLibrary.Vector_DistanceSquared` (`SceneComponent.K2_GetComponentLocation` (`Character.Mesh` (`GameplayStatics.GetPlayerCharacter` 0))) (`SceneComponent.K2_GetComponentLocation` (`/Game/Blueprints/BP_EntityPoint.DefaultSceneRoot` _array_element))) (`KismetMathLibrary.Square` (`self.SpawnRadius`)))
      (`KismetArrayLibrary.Array_Add` (`local.ValidPoints`) _array_element)))
  (if (> (`KismetArrayLibrary.Array_Length` _validpoints) 0)
    (set `self.CurrentPoint` _outitem)
    (return (`SceneComponent.K2_GetComponentLocation` (`/Game/Blueprints/BP_EntityPoint.DefaultSceneRoot` _outitem)))
    (else
      (return (-1000.0 -10000.0 -1000.0)))))

(fn `SpawnNewEntity`)

(fn `UserConstructionScript`)