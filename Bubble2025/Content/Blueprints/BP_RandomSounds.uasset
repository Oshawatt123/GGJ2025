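; Ambient sound actor that plays randomly chosen sounds at random intervals, starting after a random wait from BeginPlay.
; A self-rescheduling timer, bounded by SoundPlayMin and SoundPlayMax, picks an entry from Sounds and plays it on the Audio component.
; Each playback is stopped after a delay equal to one third of a separately rolled value from that same range.
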(event `self.ReceiveBeginPlay`
  (`KismetSystemLibrary.K2_SetTimerDelegate` (delegate `CustomEvent`) (`KismetMathLibrary.RandomFloatInRange` (`self.SoundPlayMin`) (`self.SoundPlayMax`))))

(event `CustomEvent`
  (`AudioComponent.SetSound` (`self.Audio`) (`KismetArrayLibrary.Array_Random` (`self.Sounds`)))
  (`AudioComponent.Play` (`self.Audio`) 0.0)
  (`KismetSystemLibrary.K2_SetTimerDelegate` (delegate `CustomEvent`) (`KismetMathLibrary.RandomFloatInRange` (`self.SoundPlayMin`) (`self.SoundPlayMax`)))
  (`KismetSystemLibrary.Delay` (/ (`KismetMathLibrary.RandomFloatInRange` (`self.SoundPlayMin`) (`self.SoundPlayMax`)) 3.0))
  (`AudioComponent.Stop` (`self.Audio`)))

(fn `UserConstructionScript`)